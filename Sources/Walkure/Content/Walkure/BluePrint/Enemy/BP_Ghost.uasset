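; BP_Ghost is an enemy ghost that drifts along world Y and can be targeted by a lock-on widget.
; BeginPlay randomizes its speed and direction; Tick applies that offset per frame without delta time while Stay is set, otherwise setting Stay after a delay.
; Sphere overlaps either destroy it after a delay (BP_DeleteActor) or spawn W_LockOn referencing it (BP_TargetCollision).
; LeftOrRight is unused here; clicking only prints debug text.
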(event `self.ReceiveBeginPlay`
  (set `self.GhostMoveSpeed` (`KismetMathLibrary.RandomFloatInRange` -5.0 5.0))
  (set `self.LeftOrRight?` (`KismetMathLibrary.RandomBool`)))

(event `self.ReceiveTick`
  (params (DeltaSeconds :type "Float (single-precision)"))
  (bind (_returnvalue_x _returnvalue_y _returnvalue_z) (`KismetMathLibrary.BreakVector` (`self.K2_GetActorLocation` self)))
  (if (`self.Stay`)
    (`self.K2_SetActorLocation` (`KismetMathLibrary.MakeVector` _returnvalue_x (+ _returnvalue_y (`self.GhostMoveSpeed`)) _returnvalue_z))
    (else
      (`KismetSystemLibrary.Delay` 3.0)
      (set `self.Stay` true))))

(event `self.Sphere.OnComponentBeginOverlap`
  (params (OverlappedComponent :type "PrimitiveComponent Object Reference") (OtherActor :type "Actor Object Reference") (OtherComp :type "PrimitiveComponent Object Reference") (OtherBodyIndex :type Integer) (bFromSweep :type Boolean) (SweepResult :type "HitResult Structure (by ref)"))
  (cast `/Game/Walkure/BluePrint/Enemy/BP_DeleteActor` OtherActor
    (:`then`
      (`KismetSystemLibrary.Delay` 2.0)
      (`self.K2_DestroyActor`))
    (:`CastFailed`
      (cast `/Game/Walkure/BluePrint/Enemy/BP_TargetCollision` OtherActor)
      (bind _returnvalue (`|CreateWidget` "/Game/Walkure/BluePrint/Enemy/W_LockOn.W_LockOn_C" (`GameplayStatics.GetPlayerController` 0)))
      (set `/Game/Walkure/BluePrint/Enemy/W_LockOn.P_ParameterChara` self _returnvalue)
      (`UserWidget.AddToViewport` _returnvalue 0))))

(event `self.StaticMesh.OnClicked`
  (params (TouchedComponent :type "PrimitiveComponent Object Reference") (ButtonPressed :type "Key Structure"))
  (`KismetSystemLibrary.PrintString` "Hello"))

(fn `UserConstructionScript`)