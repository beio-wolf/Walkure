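; BP_TargetCollision is an actor that follows the player's cursor position in the world while BP_PlayerCharacter's TouchBool is set.
; Each Tick it deprojects the mouse position, runs a short Visibility line trace with per-frame debug drawing, and moves itself to the hit location.
; When TouchBool is false, it parks itself at the world origin.
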(event `self.ReceiveTick`
  (params (DeltaSeconds :type "Float (single-precision)"))
  (if (`/Game/Walkure/BluePrint/Player/BP_PlayerCharacter.TouchBool` (cast `/Game/Walkure/BluePrint/Player/BP_PlayerCharacter` (`GameplayStatics.GetPlayerPawn` 0) :!pure true))
    (`self.CollisionState`)
    (else
      (`self.K2_SetActorLocation` (0.0 0.0 0.0)))))

(event `CollisionState`
  (bind (_worldlocation _worlddirection) (`PlayerController.DeprojectMousePositionToWorld` (`GameplayStatics.GetPlayerController` 0)))
  (bind _outhit (`KismetSystemLibrary.LineTraceSingle` :`Start` _worldlocation :`End` (+ _worldlocation (* _worlddirection 1000.0)) :`TraceChannel` "TraceTypeQuery1" :`DrawDebugType` "ForOneFrame"))
  (`self.K2_SetActorLocation` (`.Location` (`GameplayStatics.BreakHitResult` _outhit))))

(fn `UserConstructionScript`)