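; Game mode that triggers BP_SpawnTargetActor instances in a timed, scripted sequence.
; Tick steps through ArraySpawn, using a Delay from DelaySpawn to pace each entry, then sets ArrayIndex and fires the SpawnTarget dispatcher.
; The SpawnFlag handler, bound at BeginPlay, sets that flag on the actor at ArrayIndex in the GetAllActorsOfClass result, so targeting depends on that list's order.
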(event `self.ReceiveBeginPlay`
  (add `self.SpawnTarget` (delegate `SpawnFlag`)))

(event `SpawnFlag`
  (bind _outactors (`GameplayStatics.GetAllActorsOfClass` "/Game/Walkure/BluePrint/Enemy/BP_SpawnTargetActor.BP_SpawnTargetActor_C"))
  (set `/Game/Walkure/BluePrint/Enemy/BP_SpawnTargetActor.SpawnFlag` true (`|GetArrayItem` _outactors (`self.ArrayIndex`))))

(event `self.ReceiveTick`
  (params (DeltaSeconds :type "Float (single-precision)"))
  (if (not (== (`KismetArrayLibrary.Array_Length` (`self.ArraySpawn`)) (`self.ArrayCount`)))
    (`KismetSystemLibrary.Delay` (`|GetArrayItem` (`self.DelaySpawn`) (`self.ArrayCount`)))
    (set `self.ArrayIndex` (`|GetArrayItem` (`self.ArraySpawn`) (`self.ArrayCount`)))
    (`self.SpawnTarget`)
    (set `self.ArrayCount` (+ (`self.ArrayCount`) 1))))

(fn `UserConstructionScript`)